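; Door actor Blueprint that swings open and closed in response to OnOpen and OnClose events from its OpenDoor member.
; It stores its initial rotation at BeginPlay, and the OpenAngle timeline adds a yaw offset to that rotation each update, so the swing is relative to the placed orientation.
; Closing reverses the same timeline, and a Sound Timing event track plays the Doorlock sound at the door's location.
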(event `self.ReceiveBeginPlay`
  (set `self.Initial Rotation` (`self.K2_GetActorRotation`)))

(event `self.OpenDoor.OnOpen`
  (bind (_direction _newtrack_0) (`Timeline|Open Angle` :!label _label)
    (:`Update`
      (`self.K2_SetActorRotation` (`KismetMathLibrary.ComposeRotators` (`KismetMathLibrary.MakeRotator` 0.0 0.0 _newtrack_0) (`self.Initial Rotation`))))
    (:`Sound Timing`
      (`GameplayStatics.PlaySoundAtLocation` "/Game/door-lock.door-lock" (`self.K2_GetActorLocation`)))))

(event `self.OpenDoor.OnClose`
  (goto _label :!via `Reverse`))

(fn `UserConstructionScript`)